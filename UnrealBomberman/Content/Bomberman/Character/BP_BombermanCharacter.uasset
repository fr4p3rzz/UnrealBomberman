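; BP_BombermanCharacter is the Bomberman character Blueprint that lets the player drop bombs with the E key.
; When CanSpawn is true, it clears that flag and spawns a BP_Bomb just above the bottom of its capsule, ignoring collisions.
; It passes itself to the bomb as PlayerOwner; nothing in this Blueprint's graphs sets CanSpawn back to true.
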(event Custom|SpawnBomb
  ;[0 0 0] Spawn Bomb
  (Variables|Default|SetbCanSpawn false)
  (bind _returnvalue (Game|SpawnActorfromClass "/Game/Bomberman/Bombs/BP_Bomb.BP_Bomb_C" (Math|Transform|MakeTransform (CallFunction|GetBombSpawnLocation) "0, 0, 0" "1,1,1") "AlwaysSpawn" 0 0))
  (Variables|/Game/Bomberman/Bombs/BP_Bomb.BP_Bomb_C|SetPlayerOwner _returnvalue self))

(event EventBeginPlay)

(event Collision|EventActorBeginOverlap
  (params (OtherActor :type Actor%20Object%20Reference)))

(event EventTick
  (params (DeltaSeconds :type Float%20%28single-precision%29)))

(event Input|KeyboardEvents|E
  (params (Key :type Key%20Structure :default "None"))
  (:Pressed
    (if (Variables|Default|GetbCanSpawn)
      (CallFunction|SpawnBomb))))

(fn ConstructionScript)

(fn GetBombSpawnLocation
  (bind _returnvalue (Transformation|GetActorLocation))
  (bind (_x _y _z) (Math|Vector|BreakVector _returnvalue))
  (return (Math|Vector|MakeVector _x _y (+ (- _z (Variables|/Script/Engine.CapsuleComponent|GetCapsuleHalfHeight (Variables|Default|GetCapsuleComponent))) 2e+01))))